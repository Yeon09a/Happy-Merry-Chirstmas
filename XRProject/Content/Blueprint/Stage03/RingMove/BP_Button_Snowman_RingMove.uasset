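; Overlap-triggered snowman button for the Stage03 RingMove area that switches a snowman's animation, touch effect and sound on and off.
; Beginning an overlap activates it once, playing the animation, moving the effect and calling SnowmanB on SoundSys3.
; While nothing overlaps, Tick waits LimitTime, rechecks, then stops both and calls the Snowman sound.
; That shutdown has no IsActive check, so it repeats while idle.
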(event `self.ReceiveBeginPlay`)

(event `self.ReceiveActorBeginOverlap`
  (params (OtherActor :type "Actor Object Reference"))
  (set `self.IsClicking` true)
  (if (not (`self.IsActive`))
    (`/Game/Blueprint/Stage03/BP_Stage03_SoundSystem.SnowmanB` (`self.SoundSys3`))
    (set `self.IsActive` true)
    (`/Game/Blueprint/Stage03/Snowman/BP_Snowman.PlayAnim` (`self.Snowman`))
    (`/Game/Blueprint/Stage03/RingMove/BP_TouchEffect_Blue.MoveEffect` (`self.TouchEffect`))
    (`/Game/Blueprint/Stage03/BP_Stage03_SoundSystem.SnowmanB` (`self.SoundSys3`))))

(event `self.ReceiveActorEndOverlap`
  (params (OtherActor :type "Actor Object Reference"))
  (set `self.IsClicking` false))

(event `self.ReceiveTick`
  (params (DeltaSeconds :type "Float (single-precision)"))
  (if (not (`self.IsClicking`))
    (`KismetSystemLibrary.Delay` (`self.LimitTime`))
    (if (not (`self.IsClicking`))
      (set `self.IsActive` false)
      (`/Game/Blueprint/Stage03/Snowman/BP_Snowman.StopAnim` (`self.Snowman`))
      (`/Game/Blueprint/Stage03/RingMove/BP_TouchEffect_Blue.StopEffect` (`self.TouchEffect`))
      (`/Game/Blueprint/Stage03/BP_Stage03_SoundSystem.snowman` (`self.SoundSys3`)))))

(fn `UserConstructionScript`)