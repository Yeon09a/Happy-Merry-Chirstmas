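; Overlap-triggered button for the Stage03 RingMove area that starts and stops a train.
; On overlap begin, an inactive button becomes active, sets the spotlight intensity, moves the train, starts the touch effect and plays a train sound.
; While not overlapped, Tick waits LimitTime, then deactivates and stops train and effect if still released.
; The stop path sets the spotlight to the same intensity as the start path.
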(event `self.ReceiveBeginPlay`)

(event `self.ReceiveActorBeginOverlap`
  (params (OtherActor :type "Actor Object Reference"))
  (set `self.IsClicking` true)
  (if (not (`self.IsActive`))
    (set `self.IsActive` true)
    (`LightComponent.SetIntensity` (`SpotLight.SpotLightComponent` (`self.Spotlight`)) 200.0)
    (`/Game/Blueprint/Stage03/BP_Train.MoveTrain` (`self.Train`))
    (`/Game/Blueprint/Stage03/RingMove/BP_TouchEffect_Green.MoveEffect` (`self.TouchEffect`))
    (`/Game/Blueprint/Stage03/BP_Stage03_SoundSystem.TrainB` (`self.SoundSys3`))))

(event `self.ReceiveActorEndOverlap`
  (params (OtherActor :type "Actor Object Reference"))
  (set `self.IsClicking` false))

(event `self.ReceiveTick`
  (params (DeltaSeconds :type "Float (single-precision)"))
  (if (not (`self.IsClicking`))
    (`KismetSystemLibrary.Delay` (`self.LimitTime`))
    (if (not (`self.IsClicking`))
      (set `self.IsActive` false)
      (`LightComponent.SetIntensity` (`SpotLight.SpotLightComponent` (`self.Spotlight`)) 200.0)
      (`/Game/Blueprint/Stage03/BP_Train.StopTrain` (`self.Train`))
      (`/Game/Blueprint/Stage03/RingMove/BP_TouchEffect_Green.StopEffect` (`self.TouchEffect`)))))

(fn `UserConstructionScript`)