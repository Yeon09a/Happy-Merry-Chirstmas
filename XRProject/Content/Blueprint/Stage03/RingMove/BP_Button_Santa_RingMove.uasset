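; Overlap-driven button for the Stage03 RingMove section that starts and stops the Santa's movement, along with a touch effect.
; When an overlap begins while inactive, it marks itself active, starts Santa and the effect, and calls the SantaB sound before and after.
; While nothing is flagged as overlapping, Tick runs a LimitTime delay, then rechecks the flag before stopping both and clearing the active state.
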(event `self.ReceiveBeginPlay`)

(event `self.ReceiveActorBeginOverlap`
  (params (OtherActor :type "Actor Object Reference"))
  (set `self.IsClicking` true)
  (if (not (`self.IsActive`))
    (`/Game/Blueprint/Stage03/BP_Stage03_SoundSystem.SantaB` (`self.SoundSys3`))
    (set `self.IsActive` true)
    (`/Game/Blueprint/Stage03/BP_Santa.MoveSanta` (`self.Santa`))
    (`/Game/Blueprint/Stage03/RingMove/BP_TouchEffect_Yellow.MoveEffect` (`self.TouchEffect`))
    (`/Game/Blueprint/Stage03/BP_Stage03_SoundSystem.SantaB` (`self.SoundSys3`))))

(event `self.ReceiveActorEndOverlap`
  (params (OtherActor :type "Actor Object Reference"))
  (set `self.IsClicking` false))

(event `self.ReceiveTick`
  (params (DeltaSeconds :type "Float (single-precision)"))
  (if (not (`self.IsClicking`))
    (`KismetSystemLibrary.Delay` (`self.LimitTime`))
    (if (not (`self.IsClicking`))
      (set `self.IsActive` false)
      (`/Game/Blueprint/Stage03/BP_Santa.StopSanta` (`self.Santa`))
      (`/Game/Blueprint/Stage03/RingMove/BP_TouchEffect_Yellow.StopEffect` (`self.TouchEffect`)))))

(fn `UserConstructionScript`)