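; Stage 03 RingMove button actor that launches fireworks while something overlaps it.
; Overlap start, if inactive, activates three referenced firework actors, starts the touch effect and plays a firework sound.
; While not overlapped, Tick runs a Delay of LimitTime, then rechecks and switches the fireworks and touch effect off.
; An IsActive flag prevents retriggering until that shutdown clears it.
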(event `self.ReceiveBeginPlay`)

(event `self.ReceiveActorBeginOverlap`
  (params (OtherActor :type "Actor Object Reference"))
  (set `self.IsClicking` true)
  (if (not (`self.IsActive`))
    (set `self.IsActive` true)
    (`ActorComponent.Activate` (`NiagaraActor.NiagaraComponent` (`self.Firework00`)) true)
    (`ActorComponent.Activate` (`Actor.RootComponent` (`self.Firework01`)) true)
    (`ActorComponent.Activate` (`Actor.RootComponent` (`self.Firework02`)) true)
    (`/Game/Blueprint/Stage03/RingMove/BP_TouchEffect_Pink.MoveEffect` (`self.TouchEffect`))
    (`/Game/Blueprint/Stage03/BP_Stage03_SoundSystem.FireWorkB` (`self.SoundSys3`))))

(event `self.ReceiveActorEndOverlap`
  (params (OtherActor :type "Actor Object Reference"))
  (set `self.IsClicking` false))

(event `self.ReceiveTick`
  (params (DeltaSeconds :type "Float (single-precision)"))
  (if (not (`self.IsClicking`))
    (`KismetSystemLibrary.Delay` (`self.LimitTime`))
    (if (not (`self.IsClicking`))
      (set `self.IsActive` false)
      (`ActorComponent.Deactivate` (`NiagaraActor.NiagaraComponent` (`self.Firework00`)))
      (`ActorComponent.Deactivate` (`Actor.RootComponent` (`self.Firework01`)))
      (`ActorComponent.Deactivate` (`Actor.RootComponent` (`self.Firework02`)))
      (`/Game/Blueprint/Stage03/RingMove/BP_TouchEffect_Pink.StopEffect` (`self.TouchEffect`)))))

(fn `UserConstructionScript`)