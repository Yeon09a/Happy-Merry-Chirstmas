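; Blue touch effect actor for the Stage 03 RingMove feature that carries a dust particle effect along a spline.
; MoveEffect activates the effect and plays a timeline at the Speed rate, mapping its alpha to distance along the referenced spline actor's length to set the actor's world position.
; StopEffect deactivates the particles and halts the timeline.
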(event `self.ReceiveBeginPlay`)

(event `MoveEffect`
  (`ActorComponent.Activate` (`self.NS_DustLow_Button_Blue`) false)
  (`TimelineComponent.SetPlayRate` (`self.Timeline`) (`self.Speed`))
  (bind (_direction _moveeffect) (`Timeline|Timeline` :!label _label)
    (:`Update`
      (`self.K2_SetActorTransform` (`KismetMathLibrary.MakeTransform` (`SplineComponent.GetLocationAtDistanceAlongSpline` (`/Game/Blueprint/Stage02/BP_NiagaraSpline.Spline` (`self.Spline`)) (`KismetMathLibrary.Lerp` 0.0 (`SplineComponent.GetSplineLength` (`/Game/Blueprint/Stage02/BP_NiagaraSpline.Spline` (`self.Spline`))) _moveeffect) "World"))))))

(event `StopEffect`
  (`ActorComponent.Deactivate` (`self.NS_DustLow_Button_Blue`))
  (goto _label :!via `Stop`))

(fn `UserConstructionScript`)