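; BP_Train is a Stage03 train actor that travels along a referenced spline when triggered.
; MoveTrain plays a Timeline at a Speed-based rate, using its track to interpolate distance from zero to the spline's full length.
; Each update sets the actor's location from the spline in world space and its rotation in local space.
; StopTrain halts the Timeline.
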(event `self.ReceiveBeginPlay`)

(event `MoveTrain`
  (bind _spline (`/Game/Blueprint/Stage02/BP_NiagaraSpline.Spline` (`self.Spline`)))
  (`TimelineComponent.SetPlayRate` (`self.Timeline`) (`self.Speed`))
  (bind (_direction _newtrack_0) (`Timeline|Timeline` :!label _label)
    (:`Update`
      (bind _returnvalue (`KismetMathLibrary.Lerp` 0.0 (`SplineComponent.GetSplineLength` (`/Game/Blueprint/Stage02/BP_NiagaraSpline.Spline` (`self.Spline`))) _newtrack_0))
      (`self.K2_SetActorTransform` (`KismetMathLibrary.MakeTransform` (`SplineComponent.GetLocationAtDistanceAlongSpline` _spline _returnvalue "World") (`SplineComponent.GetRotationAtDistanceAlongSpline` _spline _returnvalue "Local"))))))

(event `StopTrain`
  (goto _label :!via `Stop`))

(fn `UserConstructionScript`)