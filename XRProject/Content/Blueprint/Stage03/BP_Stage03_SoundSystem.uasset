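; Stage 3 sound system Blueprint that plays the stage's background music and themed sounds as 2D audio.
; BeginPlay starts the main BGM, while separate events play the Santa, fire, firework, train and snowman knock sounds.
; The fire event alone is gated by an IsClicking flag and uses a Limit counter with delays, apparently intended as a cooldown.
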(event `self.ReceiveBeginPlay`
  (`self.StartStage03`))

(event `StartStage03`
  (`GameplayStatics.PlaySound2D` "/Game/Sound/Stage3BGM.Stage3BGM" 1.0 1.0 0.0 null null))

(event `SantaB`
  (`GameplayStatics.PlaySound2D` "/Game/Sound/Stage3BGMSanta.Stage3BGMSanta" 1.0 1.0 0.0 null null))

(event `FireB`
  (bind _limit (`self.limit`))
  (if (== (`self.isClicking`) true)
    (`GameplayStatics.PlaySound2D` "/Game/Sound/Stage3BGMFire.Stage3BGMFire" 1.0 1.0 0.0 null null)
    (set `self.isClicking` true)
    (while (<= _limit 0.0)
      (`/Engine/EditorBlueprintResources/StandardMacros.DecrementFloat` _limit
        (:`  `
          (`KismetSystemLibrary.Delay` 1.0))))
    (set `self.limit` 6.0)
    (else
      (`KismetSystemLibrary.Delay` (`self.limit`)))))

(event `FireWorkB`
  (`GameplayStatics.PlaySound2D` "/Game/Sound/Stage3BGMFirework.Stage3BGMFirework" 1.0 1.0 0.0 null null))

(event `TrainB`
  (`GameplayStatics.PlaySound2D` "/Game/Sound/Stage3BGMTrain.Stage3BGMTrain" 1.0 1.0 0.0 null null))

(event `SnowmanB`
  (`GameplayStatics.PlaySound2D` "/Game/Sound/Stage3BGMKnock.Stage3BGMKnock" 1.0 1.0 0.0 null null))

(fn `UserConstructionScript`)