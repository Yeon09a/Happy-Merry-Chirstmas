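; BP_TEST is a scratch test Blueprint in the OSC folder with no clear gameplay role.
; On BeginPlay it prints the negated first element of an array variable; Tick and the construction script are empty.
; Disconnected leftover nodes would hide and disable the actor, relocate it, move another object's TouchSphere to a referenced actor's location with an offset, and print that actor's transform values.
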(event `self.ReceiveTick`
  (params (DeltaSeconds :type "Float (single-precision)")))

(event `self.ReceiveBeginPlay`
  (`KismetSystemLibrary.PrintString` (`KismetStringLibrary.Conv_IntToString` (* (`|GetArrayItem` (`self.NewVar_1`)) -1))))

(fn `UserConstructionScript`)