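; BP_SensorManager converts OSC sensor touch or detection positions for one sensor into Unreal coordinates.
; While that sensor is active, Tick waits a frame, reads its data from OSCManager and rebuilds the Vector3 array.
; A linear Scale helper remaps each point from the centred sensor rect into the configured Rect, then swaps axes and negates one.
; An author note flags this Unity-to-Unreal axis conversion as untested.
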(event `self.ReceiveBeginPlay`)

(event `self.ReceiveTick`
  (params (DeltaSeconds :type "Float (single-precision)"))
  (bind _sensordataformat (`self.SensorDataFormat`))
  (bind _sensordataformat_2 (`self.SensorDataFormat`))
  (bind _rect (`self.Rect`))
  (bind _rate_scale (`self.Rate_scale`))
  (bind _rate_scale_2 (`self.Rate_scale`))
  (bind _rate_pos (`self.Rate_Pos`))
  (bind _returnvalue (`KismetMathLibrary.Conv_ByteToInt` (`self.SensorEnum`)))
  (bind _returnvalue_2 (* (`/Game/Blueprint/OSC/BP_OSCWall.PosZ` _rect) _rate_pos))
  (bind _returnvalue_3 (* (`/Game/Blueprint/OSC/BP_OSCWall.PosY` _rect) _rate_pos))
  (bind _returnvalue_4 (/ (/ (* (`/Game/Blueprint/OSC/BP_OSCWall.Height` _rect) 100.0) _rate_scale) 2.0))
  (bind _returnvalue_5 (/ (/ (* (`/Game/Blueprint/OSC/BP_OSCWall.Width` _rect) 100.0) _rate_scale) 2.0))
  (if (`|GetArrayItem` (`/Game/Blueprint/OSC/BP_SensorActiveState.SensorState` (`self.SensorActiveState`)) _returnvalue)
    (`KismetSystemLibrary.DelayUntilNextTick`)
    (bind _output_get (set `self.SensorDataFormat` (`|GetArrayItem` (`/Game/Blueprint/OSC/BP_OSCManager.SensorData` (`self.OSCManager`)) _returnvalue)))
    (`KismetArrayLibrary.Array_Clear` (`self.Vector3`))
    (for _index (range (`KismetArrayLibrary.Array_Length` (`.Position_7_D25AF78645560F9159E9BA8352663645` (break `/Game/Blueprint/OSC/S_SensorDataFormat` _output_get))))
      (`|ExecutionSequence`
        (:`then_0`
          (bind _output_x (`KismetMathLibrary.BreakVector` (`|GetArrayItem` (`.Position_7_D25AF78645560F9159E9BA8352663645` (break `/Game/Blueprint/OSC/S_SensorDataFormat` _sensordataformat_2)) _index)))
          (bind _newvalue (`self.Scale` (/ (* (`KismetMathLibrary.BreakVector2D` (break `/Game/Blueprint/OSC/S_SensorDataFormat` _sensordataformat_2)) -1.0) 2.0) (/ (`KismetMathLibrary.BreakVector2D` (break `/Game/Blueprint/OSC/S_SensorDataFormat` _sensordataformat_2)) 2.0) (- _returnvalue_3 _returnvalue_5) (+ _returnvalue_3 _returnvalue_5) _output_x)))
        (:`then_1`
          (bind (_output_x_2 _output_y) (`KismetMathLibrary.BreakVector` (`|GetArrayItem` (`.Position_7_D25AF78645560F9159E9BA8352663645` (break `/Game/Blueprint/OSC/S_SensorDataFormat` _sensordataformat)) _index)))
          (bind _newvalue_2 (`self.Scale` (/ (* (`.Y` (`KismetMathLibrary.BreakVector2D` (break `/Game/Blueprint/OSC/S_SensorDataFormat` _sensordataformat))) -1.0) 2.0) (/ (`.Y` (`KismetMathLibrary.BreakVector2D` (break `/Game/Blueprint/OSC/S_SensorDataFormat` _sensordataformat))) 2.0) (- _returnvalue_2 _returnvalue_4) (+ _returnvalue_2 _returnvalue_4) _output_y)))
        (:`then_2`
          (`KismetArrayLibrary.Array_Add` (`self.Vector3`) (`KismetMathLibrary.MakeVector` (* _newvalue_2 _rate_scale_2) (* _newvalue (* _rate_scale_2 -1.0)))))))))

(fn `Scale`
  (params (OldMin :type "Float (double-precision)") (OldMax :type "Float (double-precision)") (NewMin :type "Float (double-precision)") (NewMax :type "Float (double-precision)") (OldValue :type "Float (double-precision)"))
  (returns (NewValue :type "Float (double-precision)"))
  (return (+ (/ (* (- OldValue OldMin) (- NewMax NewMin)) (- OldMax OldMin)) NewMin)))

(fn `UserConstructionScript`)