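; BP_TouchPointGenerate maps sensor detections onto a pool of existing touch point actors each tick.
; While its sensor is active, it enables one actor per SensorManager point and disables the rest, skipping updates when points exceed the pool.
; Each TouchSphere is placed via a local transform offset from the manager's Rect, using a temporary Z lift during the move.
; An inactive sensor hides all points and disables their collision and tick.
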(event `self.ReceiveTick`
  (params (DeltaSeconds :type "Float (single-precision)"))
  (bind _sensormanager (`self.SensorManager`))
  (bind _returnvalue (`KismetArrayLibrary.Array_Length` (`/Game/Blueprint/OSC/BP_SensorManager.Vector3` (`self.SensorManager`))))
  (if (`|GetArrayItem` (`/Game/Blueprint/OSC/BP_SensorActiveState.SensorState` (`self.SensorActiveState`)) (`KismetMathLibrary.Conv_ByteToInt` (`self.SensorEnum`)))
    (if (<= (`KismetArrayLibrary.Array_Length` (`/Game/Blueprint/OSC/BP_SensorManager.Vector3` (`self.SensorManager`))) (`KismetArrayLibrary.Array_Length` (`self.TouchPoints`)))
      (for _index (range _returnvalue (`KismetArrayLibrary.Array_Length` (`self.TouchPoints`)))
        (bind _output (`|GetArrayItem` (`self.TouchPoints`) _index))
        (`self.SetActorHiddenInGame` _output true)
        (`self.SetActorEnableCollision` _output false)
        (`self.SetActorTickEnabled` _output false))
      (for _index_2 (range _returnvalue)
        (bind _output_2 (`|GetArrayItem` (`self.TouchPoints`) _index_2))
        (`self.SetActorHiddenInGame` _output_2 false)
        (`self.SetActorEnableCollision` _output_2 true)
        (`self.SetActorTickEnabled` _output_2 true)
        (bind _touchsphere (`/Game/Blueprint/OSC/BP_TouchPoint.TouchSphere` _output_2))
        (`SceneComponent.K2_SetWorldLocation` _touchsphere (+ (`self.K2_GetActorLocation` (`/Game/Blueprint/OSC/BP_SensorManager.Rect` _sensormanager)) (0.0 0.0 1000.0)) false false)
        (`SceneComponent.K2_AddLocalTransform` _touchsphere (`KismetMathLibrary.MakeTransform` (`|GetArrayItem` (`/Game/Blueprint/OSC/BP_SensorManager.Vector3` _sensormanager) _index_2) (struct) (0.5 0.5 0.3)) false false)
        (`SceneComponent.K2_SetWorldLocation` _touchsphere (- (`SceneComponent.K2_GetComponentLocation` _touchsphere) (0.0 0.0 1000.0)) false false)))
    (else
      (for _array_element (`self.TouchPoints`)
        (`self.SetActorHiddenInGame` _array_element true)
        (`self.SetActorEnableCollision` _array_element false)
        (`self.SetActorTickEnabled` _array_element false)))))

(fn `UserConstructionScript`)