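; BP_OSCManager stores data from incoming OSC sensor messages, tracking each sensor's detection area, detected object positions and active state.
; A start message sets that sensor's rect size from two floats, clears its positions and marks it active.
; Sensor messages append XY positions with zero Z, and SensorQuit marks the sensor inactive.
; State lives in arrays indexed by sensor enum; the stop-message handler is empty.
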(event `self.ReceiveBeginPlay`)

(event `GetStartMessage`
  (params (SensorEnum :type "/Game/Blueprint/OSC/E_SensorEnum Enum" :default "NewEnumerator0") (Message :type "OSCMessage Structure"))
  (bind _returnvalue (`KismetMathLibrary.Conv_ByteToInt` SensorEnum))
  (bind (_output_rectsize _output_position) (break `/Game/Blueprint/OSC/S_SensorDataFormat` (`|GetArrayItem` (`self.SensorData`) _returnvalue)))
  (bind _sensorstate (`/Game/Blueprint/OSC/BP_SensorActiveState.SensorState` (`self.SensorActiveState`)))
  ;[0.0239 1 0] 센서 연결 최신화. 방 크기 값 받기
  (bind _value (`OSCManager.GetFloat` Message))
  (bind _value_2 (`OSCManager.GetFloat` Message 1))
  (`KismetMathLibrary.Set2D` _output_rectsize _value _value_2)
  (`KismetArrayLibrary.Array_Clear` _output_position)
  (if (not (`|GetArrayItem` _sensorstate _returnvalue))
    (`KismetArrayLibrary.Array_Set` _sensorstate _returnvalue true)))

(event `GetSensorMessage`
  (params (SensorEnum :type "/Game/Blueprint/OSC/E_SensorEnum Enum" :default "NewEnumerator0") (Message :type "OSCMessage Structure"))
  (bind (_output_rectsize _output_position) (break `/Game/Blueprint/OSC/S_SensorDataFormat` (`|GetArrayItem` (`self.SensorData`) (`KismetMathLibrary.Conv_ByteToInt` SensorEnum))))
  ;[0.0239 1 0] 인식한 물체의 위치값 받기
  (bind _value (`OSCManager.GetFloat` Message))
  (bind _value_2 (`OSCManager.GetFloat` Message 1))
  (`KismetArrayLibrary.Array_Add` _output_position (`KismetMathLibrary.MakeVector` _value _value_2)))

(event `GetStopMessage`
  ;[0.0239 1 0] Comment
)

(event `SensorQuit`
  (params (SensorEnum :type "/Game/Blueprint/OSC/E_SensorEnum Enum" :default "NewEnumerator0"))
  ;[0.0239 1 0] 센서 종료 신호 받기
  (`KismetArrayLibrary.Array_Set` (`/Game/Blueprint/OSC/BP_SensorActiveState.SensorState` (`self.SensorActiveState`)) (`KismetMathLibrary.Conv_ByteToInt` SensorEnum)))

(fn `UserConstructionScript`)