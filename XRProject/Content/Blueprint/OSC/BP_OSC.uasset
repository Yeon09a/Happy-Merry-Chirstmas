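; Actor that receives OSC messages from four directional sensors (Front, Left, Right, Down) and relays them to OSCManager.
; BeginPlay creates a listening OSC server, and Tick recreates it through a resettable DoOnce whenever it is invalid.
; Each sensor's Start, Data, End and Quit address binds to its own event, which forwards to the manager with a sensor enum, except End, which sends a generic stop.
; CheckAddress is an unused address-matching helper.
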(event `self.ReceiveTick`
  (params (DeltaSeconds :type "Float (single-precision)"))
  (bind _oscserver (`self.OSCServer`))
  (bind _oscserver_2 (`self.OSCServer`))
  (`/Engine/EditorBlueprintResources/StandardMacros.IsValid` (stale _returnvalue)
    (:`Is Not Valid`
      (`/Engine/EditorBlueprintResources/StandardMacros.DoOnce` false :!label _label
        (:`Completed`
          (bind _returnvalue (`OSCManager.CreateOSCServer` (`self.Receive IPAddress`) (`self.Port`) false true "" null :!label _label_2))
          (set `self.OSCServer` _returnvalue)
          ;[1 0.8785 0] 번들로 값을 받는 것이 아닌 Server 받고 바로 Address에 의한 이벤트 바인딩 (얘가 가장 가능할 듯.  가장 유력!!/ Sequence로 모두 싹 돎)
          (`|ExecutionSequence`
            (:`then_0`
              (bind _returnvalue_2 (`OSCManager.ConvertStringToOSCAddress` "/Front/Start"))
              (`OSCServer.BindEventToOnOSCAddressPatternMatchesPath` _oscserver _returnvalue_2 (delegate `FrontStart`)))
            (:`then_1`
              (bind _returnvalue_3 (`OSCManager.ConvertStringToOSCAddress` "/Front/Data"))
              (`OSCServer.BindEventToOnOSCAddressPatternMatchesPath` _oscserver _returnvalue_3 (delegate `FrontData`)))
            (:`then_2`
              (bind _returnvalue_4 (`OSCManager.ConvertStringToOSCAddress` "/Front/End"))
              (`OSCServer.BindEventToOnOSCAddressPatternMatchesPath` _oscserver _returnvalue_4 (delegate `FrontEnd`)))
            (:`then_3`
              (bind _returnvalue_5 (`OSCManager.ConvertStringToOSCAddress` "/Front/Quit"))
              (`OSCServer.BindEventToOnOSCAddressPatternMatchesPath` _oscserver _returnvalue_5 (delegate `FrontQuit`)))
            (:`then_4`
              (bind _returnvalue_6 (`OSCManager.ConvertStringToOSCAddress` "/Left/Start"))
              (`OSCServer.BindEventToOnOSCAddressPatternMatchesPath` _oscserver _returnvalue_6 (delegate `LeftStart`)))
            (:`then_5`
              (bind _returnvalue_7 (`OSCManager.ConvertStringToOSCAddress` "/Left/Data"))
              (`OSCServer.BindEventToOnOSCAddressPatternMatchesPath` _oscserver _returnvalue_7 (delegate `LeftData`)))
            (:`then_6`
              (bind _returnvalue_8 (`OSCManager.ConvertStringToOSCAddress` "/Left/End"))
              (`OSCServer.BindEventToOnOSCAddressPatternMatchesPath` _oscserver _returnvalue_8 (delegate `LeftEnd`)))
            (:`then_7`
              (bind _returnvalue_9 (`OSCManager.ConvertStringToOSCAddress` "/Left/Quit"))
              (`OSCServer.BindEventToOnOSCAddressPatternMatchesPath` _oscserver _returnvalue_9 (delegate `LeftQuit`)))
            (:`then_8`
              (bind _returnvalue_10 (`OSCManager.ConvertStringToOSCAddress` "/Right/Start"))
              (`OSCServer.BindEventToOnOSCAddressPatternMatchesPath` _oscserver_2 _returnvalue_10 (delegate `RightStart`)))
            (:`then_9`
              (bind _returnvalue_11 (`OSCManager.ConvertStringToOSCAddress` "/Right/Data"))
              (`OSCServer.BindEventToOnOSCAddressPatternMatchesPath` _oscserver_2 _returnvalue_11 (delegate `RightData`)))
            (:`then_10`
              (bind _returnvalue_12 (`OSCManager.ConvertStringToOSCAddress` "/Right/End"))
              (`OSCServer.BindEventToOnOSCAddressPatternMatchesPath` _oscserver_2 _returnvalue_12 (delegate `RightEnd`)))
            (:`then_11`
              (bind _returnvalue_13 (`OSCManager.ConvertStringToOSCAddress` "/Right/Quit"))
              (`OSCServer.BindEventToOnOSCAddressPatternMatchesPath` _oscserver_2 _returnvalue_13 (delegate `RightQuit`)))
            (:`then_12`
              (bind _returnvalue_14 (`OSCManager.ConvertStringToOSCAddress` "/Down/Start"))
              (`OSCServer.BindEventToOnOSCAddressPatternMatchesPath` _oscserver_2 _returnvalue_14 (delegate `DownStart`)))
            (:`then_13`
              (bind _returnvalue_15 (`OSCManager.ConvertStringToOSCAddress` "/Down/Data"))
              (`OSCServer.BindEventToOnOSCAddressPatternMatchesPath` _oscserver_2 _returnvalue_15 (delegate `DownData`)))
            (:`then_14`
              (bind _returnvalue_16 (`OSCManager.ConvertStringToOSCAddress` "/Down/End"))
              (`OSCServer.BindEventToOnOSCAddressPatternMatchesPath` _oscserver_2 _returnvalue_16 (delegate `DownEnd`)))
            (:`then_15`
              (bind _returnvalue_17 (`OSCManager.ConvertStringToOSCAddress` "/Down/Quit"))
              (`OSCServer.BindEventToOnOSCAddressPatternMatchesPath` _oscserver_2 _returnvalue_17 (delegate `DownQuit`)))
            (:`then_16`
              (goto _label :!via `Reset`))))))))

(event `FrontStart`
  (params (AddressPattern :type "OSCAddress Structure (by ref)") (Message :type "OSCMessage Structure (by ref)") (IPAddress :type String) (Port :type Integer))
  ;[1 0.8785 0] 번들로 값을 받는 것이 아닌 Server 받고 바로 Address에 의한 이벤트 바인딩 (얘가 가장 가능할 듯.  가장 유력!!/ Sequence로 모두 싹 돎)
  (`/Game/Blueprint/OSC/BP_OSCManager.GetStartMessage` (`self.OSCManager`) "NewEnumerator0" Message))

(event `RightStart`
  (params (AddressPattern :type "OSCAddress Structure (by ref)") (Message :type "OSCMessage Structure (by ref)") (IPAddress :type String) (Port :type Integer))
  ;[1 0.8785 0] 번들로 값을 받는 것이 아닌 Server 받고 바로 Address에 의한 이벤트 바인딩 (얘가 가장 가능할 듯.  가장 유력!!/ Sequence로 모두 싹 돎)
  (`/Game/Blueprint/OSC/BP_OSCManager.GetStartMessage` (`self.OSCManager`) "NewEnumerator2" Message))

(event `self.ReceiveBeginPlay`
  (goto _label_2))

(event `FrontData`
  (params (AddressPattern :type "OSCAddress Structure (by ref)") (Message :type "OSCMessage Structure (by ref)") (IPAddress :type String) (Port :type Integer))
  ;[1 0.8785 0] 번들로 값을 받는 것이 아닌 Server 받고 바로 Address에 의한 이벤트 바인딩 (얘가 가장 가능할 듯.  가장 유력!!/ Sequence로 모두 싹 돎)
  (`/Game/Blueprint/OSC/BP_OSCManager.GetSensorMessage` (`self.OSCManager`) "NewEnumerator0" Message))

(event `RightData`
  (params (AddressPattern :type "OSCAddress Structure (by ref)") (Message :type "OSCMessage Structure (by ref)") (IPAddress :type String) (Port :type Integer))
  ;[1 0.8785 0] 번들로 값을 받는 것이 아닌 Server 받고 바로 Address에 의한 이벤트 바인딩 (얘가 가장 가능할 듯.  가장 유력!!/ Sequence로 모두 싹 돎)
  (`/Game/Blueprint/OSC/BP_OSCManager.GetSensorMessage` (`self.OSCManager`) "NewEnumerator2" Message))

(event `FrontEnd`
  (params (AddressPattern :type "OSCAddress Structure (by ref)") (Message :type "OSCMessage Structure (by ref)") (IPAddress :type String) (Port :type Integer))
  ;[1 0.8785 0] 번들로 값을 받는 것이 아닌 Server 받고 바로 Address에 의한 이벤트 바인딩 (얘가 가장 가능할 듯.  가장 유력!!/ Sequence로 모두 싹 돎)
  (`/Game/Blueprint/OSC/BP_OSCManager.GetStopMessage` (`self.OSCManager`)))

(event `RightEnd`
  (params (AddressPattern :type "OSCAddress Structure (by ref)") (Message :type "OSCMessage Structure (by ref)") (IPAddress :type String) (Port :type Integer))
  ;[1 0.8785 0] 번들로 값을 받는 것이 아닌 Server 받고 바로 Address에 의한 이벤트 바인딩 (얘가 가장 가능할 듯.  가장 유력!!/ Sequence로 모두 싹 돎)
  (`/Game/Blueprint/OSC/BP_OSCManager.GetStopMessage` (`self.OSCManager`)))

(event `FrontQuit`
  (params (AddressPattern :type "OSCAddress Structure (by ref)") (Message :type "OSCMessage Structure (by ref)") (IPAddress :type String) (Port :type Integer))
  ;[1 0.8785 0] 번들로 값을 받는 것이 아닌 Server 받고 바로 Address에 의한 이벤트 바인딩 (얘가 가장 가능할 듯.  가장 유력!!/ Sequence로 모두 싹 돎)
  (`/Game/Blueprint/OSC/BP_OSCManager.SensorQuit` (`self.OSCManager`) "NewEnumerator0"))

(event `RightQuit`
  (params (AddressPattern :type "OSCAddress Structure (by ref)") (Message :type "OSCMessage Structure (by ref)") (IPAddress :type String) (Port :type Integer))
  ;[1 0.8785 0] 번들로 값을 받는 것이 아닌 Server 받고 바로 Address에 의한 이벤트 바인딩 (얘가 가장 가능할 듯.  가장 유력!!/ Sequence로 모두 싹 돎)
  (`/Game/Blueprint/OSC/BP_OSCManager.SensorQuit` (`self.OSCManager`) "NewEnumerator2"))

(event `LeftStart`
  (params (AddressPattern :type "OSCAddress Structure (by ref)") (Message :type "OSCMessage Structure (by ref)") (IPAddress :type String) (Port :type Integer))
  ;[1 0.8785 0] 번들로 값을 받는 것이 아닌 Server 받고 바로 Address에 의한 이벤트 바인딩 (얘가 가장 가능할 듯.  가장 유력!!/ Sequence로 모두 싹 돎)
  (`/Game/Blueprint/OSC/BP_OSCManager.GetStartMessage` (`self.OSCManager`) "NewEnumerator1" Message))

(event `DownStart`
  (params (AddressPattern :type "OSCAddress Structure (by ref)") (Message :type "OSCMessage Structure (by ref)") (IPAddress :type String) (Port :type Integer))
  ;[1 0.8785 0] 번들로 값을 받는 것이 아닌 Server 받고 바로 Address에 의한 이벤트 바인딩 (얘가 가장 가능할 듯.  가장 유력!!/ Sequence로 모두 싹 돎)
  (`/Game/Blueprint/OSC/BP_OSCManager.GetStartMessage` (`self.OSCManager`) "NewEnumerator3" Message))

(event `LeftData`
  (params (AddressPattern :type "OSCAddress Structure (by ref)") (Message :type "OSCMessage Structure (by ref)") (IPAddress :type String) (Port :type Integer))
  ;[1 0.8785 0] 번들로 값을 받는 것이 아닌 Server 받고 바로 Address에 의한 이벤트 바인딩 (얘가 가장 가능할 듯.  가장 유력!!/ Sequence로 모두 싹 돎)
  (`/Game/Blueprint/OSC/BP_OSCManager.GetSensorMessage` (`self.OSCManager`) "NewEnumerator1" Message))

(event `DownData`
  (params (AddressPattern :type "OSCAddress Structure (by ref)") (Message :type "OSCMessage Structure (by ref)") (IPAddress :type String) (Port :type Integer))
  ;[1 0.8785 0] 번들로 값을 받는 것이 아닌 Server 받고 바로 Address에 의한 이벤트 바인딩 (얘가 가장 가능할 듯.  가장 유력!!/ Sequence로 모두 싹 돎)
  (`/Game/Blueprint/OSC/BP_OSCManager.GetSensorMessage` (`self.OSCManager`) "NewEnumerator3" Message))

(event `LeftEnd`
  (params (AddressPattern :type "OSCAddress Structure (by ref)") (Message :type "OSCMessage Structure (by ref)") (IPAddress :type String) (Port :type Integer))
  ;[1 0.8785 0] 번들로 값을 받는 것이 아닌 Server 받고 바로 Address에 의한 이벤트 바인딩 (얘가 가장 가능할 듯.  가장 유력!!/ Sequence로 모두 싹 돎)
  (`/Game/Blueprint/OSC/BP_OSCManager.GetStopMessage` (`self.OSCManager`)))

(event `DownEnd`
  (params (AddressPattern :type "OSCAddress Structure (by ref)") (Message :type "OSCMessage Structure (by ref)") (IPAddress :type String) (Port :type Integer))
  ;[1 0.8785 0] 번들로 값을 받는 것이 아닌 Server 받고 바로 Address에 의한 이벤트 바인딩 (얘가 가장 가능할 듯.  가장 유력!!/ Sequence로 모두 싹 돎)
  (`/Game/Blueprint/OSC/BP_OSCManager.GetStopMessage` (`self.OSCManager`)))

(event `LeftQuit`
  (params (AddressPattern :type "OSCAddress Structure (by ref)") (Message :type "OSCMessage Structure (by ref)") (IPAddress :type String) (Port :type Integer))
  ;[1 0.8785 0] 번들로 값을 받는 것이 아닌 Server 받고 바로 Address에 의한 이벤트 바인딩 (얘가 가장 가능할 듯.  가장 유력!!/ Sequence로 모두 싹 돎)
  (`/Game/Blueprint/OSC/BP_OSCManager.SensorQuit` (`self.OSCManager`) "NewEnumerator1"))

(event `DownQuit`
  (params (AddressPattern :type "OSCAddress Structure (by ref)") (Message :type "OSCMessage Structure (by ref)") (IPAddress :type String) (Port :type Integer))
  ;[1 0.8785 0] 번들로 값을 받는 것이 아닌 Server 받고 바로 Address에 의한 이벤트 바인딩 (얘가 가장 가능할 듯.  가장 유력!!/ Sequence로 모두 싹 돎)
  (`/Game/Blueprint/OSC/BP_OSCManager.SensorQuit` (`self.OSCManager`) "NewEnumerator3"))

(fn `UserConstructionScript`)