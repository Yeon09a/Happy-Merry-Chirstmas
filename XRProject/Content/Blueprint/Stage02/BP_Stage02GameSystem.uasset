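; Stage 02 game system Blueprint that switches five color groups of ornaments (Blue, Green, Pink, Red, Yellow) on and off.
; Every second CheckLightCount call lights one random unlit group, and TurnOffOrnament darkens a random lit one.
; An OnOrnament boolean array and an OrnamentCount track lit groups, with random picks rerolled until valid.
; Helper functions set the group's flag and call TurnOn or TurnOff on each ornament in it.
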(event `self.ReceiveBeginPlay`)

(event `CheckLightCount`
  (set `self.LightCount` (+ (`self.LightCount`) 1))
  (if (>= (`self.LightCount`) 2)
    (set `self.LightCount` 0)
    (`self.TurnOnOrnament`)))

(event `TurnOnOrnament`
  (bind _onornament (`self.OnOrnament`))
  (if (< (`self.OrnamentCount`) 5)
    (set `self.OrnamentCount` (+ (`self.OrnamentCount`) 1))
    (bind _output_get (set `self.RandomIndex` (`KismetMathLibrary.RandomInteger` (`KismetArrayLibrary.Array_Length` _onornament)) :!label _label))
    (if (`|GetArrayItem` _onornament _output_get)
      (goto _label)
      (else
        (switch `int` _output_get
          (:`0`
            (`self.TurnOnOrnaments` (`self.Blue`)))
          (:`1`
            (`self.TurnOnOrnaments` (`self.Green`) 1))
          (:`2`
            (`self.TurnOnOrnaments` (`self.Pink`) 2))
          (:`3`
            (`self.TurnOnOrnaments` (`self.Red`) 3))
          (:`4`
            (`self.TurnOnOrnaments` (`self.Yellow`) 4)))))))

(event `TurnOffOrnament`
  (bind _onornament (`self.OnOrnament`))
  (if (> (`self.OrnamentCount`) 0)
    (set `self.OrnamentCount` (- (`self.OrnamentCount`) 1))
    (bind _output_get (set `self.RandomOffIndex` (`KismetMathLibrary.RandomInteger` (`KismetArrayLibrary.Array_Length` _onornament)) :!label _label_2))
    (if (`|GetArrayItem` _onornament _output_get)
      (switch `int` _output_get
        (:`0`
          (`self.TurnOffOrnaments` (`self.Blue`)))
        (:`1`
          (`self.TurnOffOrnaments` (`self.Green`) 1))
        (:`2`
          (`self.TurnOffOrnaments` (`self.Pink`) 2))
        (:`3`
          (`self.TurnOffOrnaments` (`self.Red`) 3))
        (:`4`
          (`self.TurnOffOrnaments` (`self.Yellow`) 4)))
      (else
        (goto _label_2)))))

(fn `TurnOffOrnaments`
  (params (Ornament :type "Array of /Game/Blueprint/Stage02/BP_Ornament Object Reference") (OrnamentNum :type Integer))
  (`KismetArrayLibrary.Array_Set` (`self.OnOrnament`) OrnamentNum)
  (for _array_element Ornament
    (`/Game/Blueprint/Stage02/BP_Ornament.TurnOff` _array_element)))

(fn `TurnOnOrnaments`
  (params (Ornaments :type "Array of /Game/Blueprint/Stage02/BP_Ornament Object Reference") (OnamenrtNum :type Integer))
  (`KismetArrayLibrary.Array_Set` (`self.OnOrnament`) OnamenrtNum true)
  (for _array_element Ornaments
    (`/Game/Blueprint/Stage02/BP_Ornament.TurnOn` _array_element)))

(fn `UserConstructionScript`)