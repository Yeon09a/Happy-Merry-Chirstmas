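; BP_Ornament00 is a Stage 02 ornament with a swirl sphere mesh that can be switched between lit and unlit looks.
; The construction script stores the swirl base-color material as the original and starts the ornament unlit.
; TurnOnLight and TurnOffLight each call the parent implementation, then swap the sphere's material to the pink ornament material or back to the original.
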(fn `TurnOffLight`
  (`parent.TurnOffLight`)
  (`PrimitiveComponent.SetMaterial` (`self.all_swirl_Sphere01`) 0 (`self.OriMaterial`)))

(fn `TurnOnLight`
  (`parent.TurnOnLight`)
  (`PrimitiveComponent.SetMaterial` (`self.all_swirl_Sphere01`) 0 "/Game/Material/Stage02/Ornament/M_Stage02Ornament_Pink.M_Stage02Ornament_Pink"))

(fn `UserConstructionScript`
  (set `self.OriMaterial` "/Game/Stage02Map/Asset/christmas-ornaments/textures/swirl_swirl_Sphere03_BaseColor_Mat.swirl_swirl_Sphere03_BaseColor_Mat")
  (`self.TurnOffLight`))