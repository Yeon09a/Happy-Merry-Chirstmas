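; BP_Stocking is a Stage02 actor that travels along the spline of a referenced actor.
; On BeginPlay it plays a timeline at a rate set by Speed, mapping the Move track onto the spline's length.
; Each update sets the actor's transform from world-space location and local-space rotation at that distance, with scale taken from a Scale variable.
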(event `self.ReceiveBeginPlay`
  (bind _spline (`/Game/Blueprint/Stage02/BP_NiagaraSpline.Spline` (`self.Spline`)))
  (`TimelineComponent.SetPlayRate` (`self.Timeline`) (`self.Speed`))
  (bind (_direction _move) (`Timeline|Timeline`)
    (:`Update`
      (bind _returnvalue (`KismetMathLibrary.Lerp` 0.0 (`SplineComponent.GetSplineLength` (`/Game/Blueprint/Stage02/BP_NiagaraSpline.Spline` (`self.Spline`))) _move))
      (`self.K2_SetActorTransform` (`KismetMathLibrary.MakeTransform` (`SplineComponent.GetLocationAtDistanceAlongSpline` _spline _returnvalue "World") (`SplineComponent.GetRotationAtDistanceAlongSpline` _spline _returnvalue "Local") (`self.Scale`))))))

(fn `UserConstructionScript`)