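; BP_Ornament04 is the white star ornament in Stage 02, with a lit and an unlit state.
; It overrides TurnOnLight and TurnOffLight, calling the parent before swapping the AllStar mesh material.
; Lighting it also activates the white Niagara effect; turning it off only restores the original material here.
; The construction script stores that original material and starts the ornament unlit.
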(event `self.ReceiveBeginPlay`)

(fn `TurnOffLight`
  (`parent.TurnOffLight`)
  (`PrimitiveComponent.SetMaterial` (`self.all_Star`) 0 (`self.OriMaterial`)))

(fn `TurnOnLight`
  (`parent.TurnOnLight`)
  (`ActorComponent.Activate` (`self.NS_Ornament_White`) true)
  (`PrimitiveComponent.SetMaterial` (`self.all_Star`) 0 "/Game/Material/Stage02/Ornament/M_Stage02Ornament_White.M_Stage02Ornament_White"))

(fn `UserConstructionScript`
  (set `self.OriMaterial` "/Game/Stage02Map/Asset/christmas-ornaments/textures/star_Star1_BaseColor_Mat.star_Star1_BaseColor_Mat")
  (`self.TurnOffLight`))