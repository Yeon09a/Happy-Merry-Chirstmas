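; BP_Ornament03 is a Stage 02 ornament Blueprint that switches between an unlit and a lit look.
; It overrides the parent's TurnOnLight and TurnOffLight, then swaps material slot 1 on AllBool1 between the blue ornament material and its original base material.
; The construction script stores that original material and starts the ornament turned off.
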(fn `TurnOffLight`
  (`parent.TurnOffLight`)
  (`PrimitiveComponent.SetMaterial` (`self.all_bool1`) 1 (`self.OriMaterial`)))

(fn `TurnOnLight`
  (`parent.TurnOnLight`)
  (`PrimitiveComponent.SetMaterial` (`self.all_bool1`) 1 "/Game/Material/Stage02/Ornament/M_Stage02Ornament_Blue.M_Stage02Ornament_Blue"))

(fn `UserConstructionScript`
  (set `self.OriMaterial` "/Game/Stage02Map/Asset/christmas-ornaments/textures/bool_bool1_BaseColor_Mat.bool_bool1_BaseColor_Mat")
  (`self.TurnOffLight`))