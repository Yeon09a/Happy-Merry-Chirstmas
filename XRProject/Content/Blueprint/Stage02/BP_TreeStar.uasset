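; BP_TreeStar is the Stage 02 tree star that lights up when an actor overlaps it and ends the stage.
; The construction script puts a dynamic yellow light material on a mesh with emissive at zero.
; Overlap activates the yellow Niagara effect, raises the emissive through TurnOn and calls the sound system's BrightTree.
; After a delay, it calls EndStage02 on the sound system and CallLevelMove on the game system.
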(event `self.ReceiveBeginPlay`)

(event `self.ReceiveActorBeginOverlap`
  (params (OtherActor :type "Actor Object Reference"))
  (bind _stage02soundsys (`self.Stage02SoundSys`))
  (`ActorComponent.Activate` (`self.NS_TreeYellow`) false)
  (`self.TurnOn`)
  (`/Game/Blueprint/Stage02/BP_Stage02_SoundSystem.BrightTree` _stage02soundsys)
  (`KismetSystemLibrary.Delay` 10.0)
  (`/Game/Blueprint/Stage02/BP_Stage02_SoundSystem.EndStage02` _stage02soundsys)
  (`/Game/Blueprint/Stage02/BP_Stage02GameSystem_2Sides.LevelMove` (`self.Stage02GameSystem`)))

(fn `TurnOn`
  (`MaterialInstanceDynamic.SetScalarParameterValue` (`self.MaterialCopy`) "EmissiveValue" 20.0))

(fn `UserConstructionScript`
  (bind _returnvalue (`PrimitiveComponent.CreateDynamicMaterialInstance` (`self.Object_15`) 0 "/Game/Material/Stage02/M_Stage02Light_Yellow.M_Stage02Light_Yellow" "None"))
  (bind _output_get (set `self.MaterialCopy` _returnvalue))
  (`MaterialInstanceDynamic.SetScalarParameterValue` _output_get "EmissiveValue" 0.0))