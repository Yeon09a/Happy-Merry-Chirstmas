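; BP_Light is a Stage 02 star light that flickers out and is fixed when an actor tagged "Touchpoint" overlaps it while off.
; TurnOff alternates the star mesh's yellow and off materials through timed delays, then fires a red burst and flags it off.
; A fix plays sound and yellow Niagara effects, reports its LightNum to the Garland and turns on ornaments through the stage system.
; TurnOnFinal relights it with effects only.
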(event `self.ReceiveActorBeginOverlap`
  (params (OtherActor :type "Actor Object Reference"))
  (bind _ns_lightline_yellow (`self.NS_LightLine_Yellow`))
  (if (`self.ActorHasTag` OtherActor "Touchpoint")
    (if (`self.IsOff`)
      (set `self.IsOff` false)
      (`self.TurnOn`)
      (`/Game/Blueprint/Stage02/BP_Stage02_SoundSystem.LightFix` (`self.SoundSys2`))
      (`ActorComponent.Activate` (`self.N_LightBlast_Yellow`) true)
      (`ActorComponent.Deactivate` _ns_lightline_yellow)
      (`ActorComponent.Activate` _ns_lightline_yellow false)
      (`/Game/Blueprint/Stage02/BP_Stage02GameSystem_2Sides.TurnOnOrnaments` (`self.Stage02GameSystem`)))))

(event `TurnOn`
  (`self.TurnOnLight`)
  (`/Game/Blueprint/Stage02/BP_Garland.LightOffCheck` (`self.Garland`) (`self.LightNum`)))

(event `TurnOnFinal`
  (`self.TurnOnLight`)
  (`ActorComponent.Activate` (`self.NS_LightLine_Yellow`) true)
  (`ActorComponent.Activate` (`self.N_LightBlast_Yellow`) true))

(event `TurnOff`
  (bind _effecttime (`self.EffectTime`))
  (bind _effecttime_2 (`self.EffectTime`))
  (bind _effecttime_3 (`self.EffectTime`))
  (`self.TurnOffLight`)
  (`KismetSystemLibrary.Delay` _effecttime_2)
  (`self.TurnOnLight`)
  (`KismetSystemLibrary.Delay` _effecttime_2)
  (`self.TurnOffLight`)
  (`KismetSystemLibrary.Delay` _effecttime_3)
  (`self.TurnOnLight`)
  (`KismetSystemLibrary.Delay` _effecttime_3)
  (`self.TurnOffLight`)
  (`KismetSystemLibrary.Delay` _effecttime)
  (`self.TurnOnLight`)
  (`KismetSystemLibrary.Delay` _effecttime)
  (`ActorComponent.Activate` (`self.N_LightBlast_Star_Red`) false)
  (`self.TurnOffLight`)
  (`/Game/Blueprint/Stage02/BP_Stage02_SoundSystem.LightOut` (`self.SoundSys2`))
  (set `self.IsOff` true))

(fn `TurnOffLight`
  (`PrimitiveComponent.SetMaterial` (`self.star_Star001`) 0 "/Game/Material/Stage02/M_Stage02Light_Off.M_Stage02Light_Off"))

(fn `TurnOnLight`
  (`PrimitiveComponent.SetMaterial` (`self.star_Star001`) 0 (`self.MaterialCopy`)))

(fn `UserConstructionScript`
  (set `self.MaterialCopy` "/Game/Material/Stage02/M_Stage02Light_Yellow.M_Stage02Light_Yellow"))