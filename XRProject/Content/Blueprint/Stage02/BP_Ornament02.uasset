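; BP_Ornament02 is a Stage02 ornament that switches between an unlit look and a red lit look, extending its parent's light toggle.
; Construction caches the round belt's base material and starts the ornament turned off.
; TurnOnLight calls the parent, activates the red Niagara effect and swaps AllRoundBelt to the red material.
; TurnOffLight calls the parent and restores the cached material, without explicitly deactivating the effect.
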(fn `TurnOffLight`
  (`parent.TurnOffLight`)
  (`PrimitiveComponent.SetMaterial` (`self.all_round_belt`) 0 (`self.OriMaterial`)))

(fn `TurnOnLight`
  (`parent.TurnOnLight`)
  (`ActorComponent.Activate` (`self.NS_Ornament_Red`) true)
  (`PrimitiveComponent.SetMaterial` (`self.all_round_belt`) 0 "/Game/Material/Stage02/Ornament/M_Stage02Ornament_Red.M_Stage02Ornament_Red"))

(fn `UserConstructionScript`
  (set `self.OriMaterial` "/Game/Stage02Map/Asset/christmas-ornaments/textures/rb_round_belt_BaseColor_Mat.rb_round_belt_BaseColor_Mat")
  (`self.TurnOffLight`))