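; BP_Stage02GameSystem_2Sides manages Stage 02's ornament-lighting progress, tracking lit and unlit ornaments in two arrays with a running count.
; TurnOnOrnaments lights up to two random unlit ornaments, while TurnOffOrnaments reverts two random lit ones unless the count is zero.
; Both move ornaments between the arrays.
; Reaching the count threshold triggers Finish, which stops Garland play, plays a sound, calls Garland's finish and lights every ornament.
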(event `self.ReceiveBeginPlay`)

(event `TurnOnOrnaments`
  (for _ (range 1 3)
    (set `self.OnCount` (+ (`self.OnCount`) 1))
    (bind _output_get (set `self.RandomIndexOn` (`KismetMathLibrary.RandomInteger` (`KismetArrayLibrary.Array_Length` (`self.OffOrnaments`)))))
    (bind _output (`|GetArrayItem` (`self.OffOrnaments`) _output_get))
    (`/Game/Blueprint/Stage02/BP_Ornament.TurnOn` _output)
    (`KismetArrayLibrary.Array_Add` (`self.OnOrnaments`) _output)
    (`KismetArrayLibrary.Array_Remove` (`self.OffOrnaments`) _output_get)
    (if (>= (`self.OnCount`) 25)
      (break)))
  ;[1 1 1] 종료 조건
  (if (>= (`self.OnCount`) 25)
    (`self.Finish`)))

(event `TurnOffOrnaments`
  (if (<= (`self.OnCount`) 0)
    (goto _label :!via `Break`)
    (else
      (for _ (range 1 3) :!label _label
        (set `self.OnCount` (- (`self.OnCount`) 1))
        (bind _output_get (set `self.RandomIndexOff` (`KismetMathLibrary.RandomInteger` (`KismetArrayLibrary.Array_Length` (`self.OnOrnaments`)))))
        (bind _output (`|GetArrayItem` (`self.OnOrnaments`) _output_get))
        (`/Game/Blueprint/Stage02/BP_Ornament.TurnOff` _output)
        (`KismetArrayLibrary.Array_Add` (`self.OffOrnaments`) _output)
        (`KismetArrayLibrary.Array_Remove` (`self.OnOrnaments`) _output_get)))))

(event `Finish`
  (set `/Game/Blueprint/Stage02/BP_Garland.IsPlaying` false (`self.Garland`))
  (`GameplayStatics.PlaySound2D` null 1.0 1.0 0.0 null (`self.SoundSys2`))
  (`/Game/Blueprint/Stage02/BP_Garland.Finish` (`self.Garland`))
  (for _array_element (`self.Ornaments`)
    (`/Game/Blueprint/Stage02/BP_Ornament.TurnOn` _array_element)))

(fn `UserConstructionScript`)