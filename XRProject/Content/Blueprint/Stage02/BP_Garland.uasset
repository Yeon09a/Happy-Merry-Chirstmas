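; Stage 02 garland actor that runs a light-relighting game by repeatedly switching off random bulbs.
; After a startup delay it turns off five distinct lights, tracked in a boolean array and counter.
; A delayed Tick darkens five more once at most one stays off, with LightOffCheck clearing relit entries.
; Finish and FinishGarland stop play, disable light sphere collision and trigger each light's final on state.
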(event `self.ReceiveBeginPlay`
  (`KismetSystemLibrary.Delay` 3.3)
  (`self.TurnOff`)
  (set `self.IsPlaying` true))

(event `self.ReceiveTick`
  (params (DeltaSeconds :type "Float (single-precision)"))
  (`KismetSystemLibrary.Delay` 2.0)
  (if (and (`self.IsPlaying`) (<= (`self.CurOffLight`) 1))
    (`self.TurnOffLights` 5)))

(event `TurnOff`
  (`self.TurnOffLights` 5))

(event `Finish`
  (set `self.IsPlaying` false)
  (`self.SetActorTickEnabled` false)
  (for _array_element (`self.Lights`)
    (`PrimitiveComponent.SetCollisionEnabled` (`/Game/Blueprint/Stage02/BP_Light.Sphere` _array_element) "NoCollision")
    (`/Game/Blueprint/Stage02/BP_Light.TurnOnFinal` _array_element)))

(event `LightOffCheck`
  (params (LightNum :type Integer))
  (set `self.CurOffLight` (- (`self.CurOffLight`) 1))
  (`KismetArrayLibrary.Array_Set` (`self.OffLights`) LightNum))

(fn `FinishGarland`
  (`self.SetActorTickEnabled` false)
  (set `self.IsPlaying` false)
  (for _array_element (`self.AllLights`)
    (`PrimitiveComponent.SetCollisionEnabled` (`/Game/Blueprint/Stage02/BP_Light.Sphere` _array_element) "NoCollision")
    (`/Game/Blueprint/Stage02/BP_Light.TurnOnFinal` _array_element)))

(fn `TurnOffLights`
  (params (LightCount :type Integer))
  (bind _offlights (`self.OffLights`))
  (while (< (`self.OffLight`) LightCount)
    (bind _output_get (set `self.RandomLightNum` (`KismetMathLibrary.RandomInteger` (`KismetArrayLibrary.Array_Length` _offlights))))
    (if (not (`|GetArrayItem` _offlights _output_get))
      (set `self.OffLight` (+ (`self.OffLight`) 1))
      (set `self.CurOffLight` (+ (`self.CurOffLight`) 1))
      (`KismetArrayLibrary.Array_Set` (`self.OffLights`) _output_get true)
      (`/Game/Blueprint/Stage02/BP_Light.TurnOff` (`|GetArrayItem` (`self.Lights`) _output_get))))
  (set `self.OffLight` 0))

(fn `UserConstructionScript`)