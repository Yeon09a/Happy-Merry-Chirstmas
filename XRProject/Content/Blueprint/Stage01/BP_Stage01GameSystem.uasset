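; Stage 01 game system actor that runs a star-collecting round, ending once 30 stars are found.
; ActiveStar moves the next pre-placed star to a random free position, rerolling occupied slots, and activates it.
; GameStart and a Delay-throttled Tick keep seven stars active until 30 are used.
; GetStar frees the slot, spawns a color-matched particle and triggers FinishGame, which stops Tick and resets counters.
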(event `self.ReceiveBeginPlay`
  (`self.GameStart`))

(event `self.ReceiveTick`
  (params (DeltaSeconds :type "Float (single-precision)"))
  ;[1 1 1] 4초마다 별 활성화(게임 끝나면 비활성화)
  (`KismetSystemLibrary.Delay` 2.0)
  (while (and (< (`self.ActiveStarCount`) 7) (< (`self.StarIndex`) 30))
    (`self.ActiveStar`)))

(event `GameStart`
  ;[1 1 1] 게임 시작
  (while (< (`self.ActiveStarCount`) 7)
    (`self.ActiveStar`)))

(event `ActiveGame`
  ;[1 1 1] Game 활성화
  (`self.SetActorTickEnabled` true)
  (`self.SetActorHiddenInGame` false))

(event `GetStar`
  (params (StarPos :type Integer) (Color :type "/Game/Blueprint/Stage01/E_ColorEnum Enum" :default "NewEnumerator0"))
  (bind _spawnparticle (`self.SpawnParticle`))
  ;[1 1 1] 별을 얻음
  (set `self.ActiveStarCount` (- (`self.ActiveStarCount`) 1))
  (set `self.FindStarCount` (+ (`self.FindStarCount`) 1))
  (`KismetArrayLibrary.Array_Set` (`self.NotEmptyPos`) StarPos)
  (switch `/Game/Blueprint/Stage01/E_ColorEnum` Color
    (:`NewEnumerator0`
      (`/Game/Blueprint/Stage01/BP_SpawnParticle.SpawnBlue` _spawnparticle))
    (:`NewEnumerator1`
      (`/Game/Blueprint/Stage01/BP_SpawnParticle.SpawnGreen` _spawnparticle))
    (:`NewEnumerator2`
      (`/Game/Blueprint/Stage01/BP_SpawnParticle.SpawnPink` _spawnparticle)))
  (if (>= (`self.FindStarCount`) 30)
    (`self.FinishGame`)))

(event `FinishGame`
  ;[1 1 1] 게임 끝
  (`self.SetActorTickEnabled` false)
  (`self.SetActorHiddenInGame` false)
  (`KismetSystemLibrary.Delay` 2.0)
  (set `self.ActiveStarCount` 0)
  (set `self.FindStarCount` 0)
  (set `self.RandomIndex` 0)
  (set `self.StarIndex` 0))

(fn `ActiveStar`
  (bind _output (`|GetArrayItem` (`self.Stars`) (`self.StarIndex`)))
  (bind _output_get (set `self.RandomIndex` (`KismetMathLibrary.RandomInteger` (`KismetArrayLibrary.Array_Length` (`self.Pos`))) :!label _label))
  (if (`|GetArrayItem` (`self.NotEmptyPos`) _output_get)
    (goto _label)
    (else
      (`self.K2_SetActorLocation` _output (`|GetArrayItem` (`self.Pos`) _output_get) false false)
      (`/Game/Blueprint/Stage01/BP_Star.SetActive` _output)
      (`KismetArrayLibrary.Array_Set` (`self.NotEmptyPos`) _output_get true)
      (set `/Game/Blueprint/Stage01/BP_Star.SpawnPosIndex` _output_get _output)
      (set `self.StarIndex` (+ (`self.StarIndex`) 1))
      (set `self.ActiveStarCount` (+ (`self.ActiveStarCount`) 1)))))

(fn `UserConstructionScript`)