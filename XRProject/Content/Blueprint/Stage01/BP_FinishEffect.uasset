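; BP_FinishEffect is a Stage01 effect actor that switches three white fireworks effects on and off, apparently for a finish moment.
; StartEffect activates the three fireworks components without reset, and FinishEffect deactivates them.
; It has no logic of its own on BeginPlay, overlap or Tick, so both events rely on being called from elsewhere.
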(event `StartEffect`
  (`|ExecutionSequence`
    (:`then_0`
      (`ActorComponent.Activate` (`self.NS_Fireworks_White`) false))
    (:`then_1`
      (`ActorComponent.Activate` (`self.NS_Fireworks_White1`) false))
    (:`then_2`
      (`ActorComponent.Activate` (`self.NS_Fireworks_White2`) false))))

(event `FinishEffect`
  (`|ExecutionSequence`
    (:`then_0`
      (`ActorComponent.Deactivate` (`self.NS_Fireworks_White`)))
    (:`then_1`
      (`ActorComponent.Deactivate` (`self.NS_Fireworks_White1`)))
    (:`then_2`
      (`ActorComponent.Deactivate` (`self.NS_Fireworks_White2`)))))

(fn `UserConstructionScript`)