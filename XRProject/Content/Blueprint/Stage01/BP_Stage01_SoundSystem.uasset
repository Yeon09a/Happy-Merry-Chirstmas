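; Stage 01 sound controller that plays the stage music, star-found cues and a map-change sound.
; StartStage01 plays the BGM, then replays it every five seconds while ChangeLevel.NowLevel equals PareLevel.
; When they differ, it applies a zero-volume sound mix class override and plays the Changemap sound.
; Separate events play the blue, red and green star-found sounds as 2D one-shots.
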(event `self.ReceiveBeginPlay`)

(event `StartStage01`
  ;[1 1 1] 스테이지 시작
  (`GameplayStatics.PlaySound2D` "/Game/Sound/Stage1BGM.Stage1BGM" 1.0 1.0 0.0 null null)
  (while (== (`/Game/Blueprint/BP_ChangeLevel_2Sides.nowLevel` (`self.ChangeLevel`)) (`self.pareLevel`))
    (`KismetSystemLibrary.Delay` 5.0)
    (`GameplayStatics.PlaySound2D` "/Game/Sound/Stage1BGM.Stage1BGM" 1.0 1.0 0.0 null null))
  (`GameplayStatics.SetSoundMixClassOverride` null null 0.0 0.0 0.0)
  (`GameplayStatics.PlaySound2D` "/Game/Sound/changemap.changemap" 1.0 1.0 0.0 null null))

(event `FindStarBlue`
  ;[1 1 1] 별 찾음
  (`GameplayStatics.PlaySound2D` "/Game/Sound/Stage1FindBlue.Stage1FindBlue" 1.0 1.0 0.0 null null))

(event `FindStarRed`
  ;[1 1 1] 별 찾음
  (`GameplayStatics.PlaySound2D` "/Game/Sound/Stage1FindRed.Stage1FindRed" 1.0 1.0 0.0 null null))

(event `FindStarGreen`
  ;[1 1 1] 별 찾음
  (`GameplayStatics.PlaySound2D` "/Game/Sound/Stage1FindGreen.Stage1FindGreen" 1.0 1.0 0.0 null null))

(fn `UserConstructionScript`)