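; BP_Deer is a Stage01 animal actor that walks a deer along splines and periodically pauses it to look around.
; A timeline at a configurable play rate drives position and rotation along the current spline, then swaps it through AnimalControl and restarts.
; Tick waits a randomized Delay, then sets IsLooking on the one- or two-sided anim instance and stops the timeline.
; The Move event resumes movement.
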(event `self.ReceiveBeginPlay`
  (bind _spline (`/Game/Blueprint/Stage01/Animal/BP_AnimalSpline.Spline` (`self.Spline`)))
  (`TimelineComponent.SetPlayRate` (`self.Timeline`) (`self.Speed`))
  (bind (_direction _movedeer) (`Timeline|Timeline` :!label _label)
    (:`Update`
      (bind _returnvalue (`KismetMathLibrary.Lerp` 0.0 (`SplineComponent.GetSplineLength` (`/Game/Blueprint/Stage01/Animal/BP_AnimalSpline.Spline` (`self.Spline`))) _movedeer))
      (`self.K2_SetActorTransform` (`KismetMathLibrary.MakeTransform` (`SplineComponent.GetLocationAtDistanceAlongSpline` _spline _returnvalue "World") (`SplineComponent.GetRotationAtDistanceAlongSpline` _spline _returnvalue "Local"))))
    (:`Finished`
      (`self.MoveDone`)
      (goto _label :!via `PlayFromStart`))))

(event `self.ReceiveTick`
  (params (DeltaSeconds :type "Float (single-precision)"))
  (bind _returnvalue (`SkeletalMeshComponent.GetAnimInstance` (`self.SK_DeerStag`)))
  (bind _returnvalue_2 (`KismetMathLibrary.Conv_IntToDouble` (+ (`KismetMathLibrary.RandomInteger` 5) (`self.AnimTime`))))
  (if (`self.Is2Side`)
    (bind _asbp_deer_anim_2sides (cast `/Game/Blueprint/Stage01/Animal/BP_DeerAnim_2Sides` _returnvalue))
    (if (not (`/Game/Blueprint/Stage01/Animal/BP_DeerAnim_2Sides.IsLooking` _asbp_deer_anim_2sides))
      (`KismetSystemLibrary.Delay` _returnvalue_2)
      (set `/Game/Blueprint/Stage01/Animal/BP_DeerAnim_2Sides.IsLooking` true _asbp_deer_anim_2sides)
      (goto _label :!via `Stop`))
    (else
      (bind _asbp_deer_anim (cast `/Game/Blueprint/Stage01/Animal/BP_DeerAnim` _returnvalue))
      (if (not (`/Game/Blueprint/Stage01/Animal/BP_DeerAnim.IsLooking` _asbp_deer_anim))
        (`KismetSystemLibrary.Delay` _returnvalue_2)
        (set `/Game/Blueprint/Stage01/Animal/BP_DeerAnim.IsLooking` true _asbp_deer_anim)
        (goto _label :!via `Stop`)))))

(event `Move`
  (goto _label))

(event `MoveDone`
  (bind _animalcontrol (`self.AnimalControl`))
  (`/Game/Blueprint/Stage01/Animal/BP_AnimalControl.UnuseSpline` _animalcontrol (`self.SplineIndex`))
  (bind (_spline _splineindex) (`/Game/Blueprint/Stage01/Animal/BP_AnimalControl.ChooseSpline` _animalcontrol))
  (set `self.SplineIndex` _splineindex)
  (set `self.Spline` _spline))

(fn `UserConstructionScript`)