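; BP_AnimalControl is a Stage01 animal manager that hands out splines, presumably animal paths, so that no two users share one.
; ChooseSpline rerolls a random index among three until it finds a free one, flags it in UseSpline and returns the spline with its index.
; UnuseSpline clears that flag to free the slot.
; The reroll loop has no exit when all three are taken, and the event graph is empty.
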(fn `ChooseSpline`
  (returns (Spline :type "/Game/Blueprint/Stage01/Animal/BP_AnimalSpline Object Reference") (SplineIndex :type Integer))
  (bind _randomindex (`self.RandomIndex`))
  (set `self.RandomIndex` (`KismetMathLibrary.RandomInteger` 3) :!label _label)
  (if (`|GetArrayItem` (`self.UseSpline`) _randomindex)
    (goto _label)
    (else
      (`KismetArrayLibrary.Array_Set` (`self.UseSpline`) _randomindex true)
      (return (`|GetArrayItem` (`self.Spline`) _randomindex) _randomindex))))

(fn `UnuseSpline`
  (params (SplineIndex :type Integer))
  (`KismetArrayLibrary.Array_Set` (`self.UseSpline`) SplineIndex))

(fn `UserConstructionScript`)