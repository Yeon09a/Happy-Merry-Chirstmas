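; BP_Star is a collectible star actor for Stage 01 that reports its StarNum to Stage01GameSystem on overlap, then deactivates itself.
; The construction script starts it hidden, with collision and tick disabled.
; SetActive and SetInActive events toggle visibility, collision and tick together, so the star is switched on and off without spawning or destroying it.
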(event `self.ReceiveBeginPlay`)

(event `self.ReceiveActorBeginOverlap`
  (params (OtherActor :type "Actor Object Reference"))
  (`/Game/Blueprint/Stage01/BP_Stage01GameSystem.GetStar` (`self.Stage01GameSystem`) (`self.StarNum`))
  (`self.SetInActive`))

(event `SetActive`
  (`self.SetActorHiddenInGame` false)
  (`self.SetActorEnableCollision` true)
  (`self.SetActorTickEnabled` true))

(event `SetInActive`
  (`self.SetActorEnableCollision` false)
  (`self.SetActorHiddenInGame` true)
  (`self.SetActorTickEnabled` false))

(fn `UserConstructionScript`
  (`self.SetActorEnableCollision` false)
  (`self.SetActorHiddenInGame` true)
  (`self.SetActorTickEnabled` false))