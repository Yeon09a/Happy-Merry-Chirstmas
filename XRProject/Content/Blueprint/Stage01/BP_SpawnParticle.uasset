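; BP_SpawnParticle is a Stage 01 Blueprint that plays pink, blue or green particle effects on demand.
; Three custom events, SpawnPink, SpawnBlue and SpawnGreen, each re-trigger their own color's particle component by calling Deactivate, then Activate without the reset flag.
; It has no active BeginPlay, overlap, Tick or construction logic, so those effects are triggered only through these events.
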(event `SpawnPink`
  (bind _ns_particle_pink (`self.NS_Particle_Pink`))
  (`ActorComponent.Deactivate` _ns_particle_pink)
  (`ActorComponent.Activate` _ns_particle_pink false))

(event `SpawnBlue`
  (bind _ns_particle_blue (`self.NS_Particle_Blue`))
  (`ActorComponent.Deactivate` _ns_particle_blue)
  (`ActorComponent.Activate` _ns_particle_blue false))

(event `SpawnGreen`
  (bind _ns_partlcle_green (`self.NS_Partlcle_Green`))
  (`ActorComponent.Deactivate` _ns_partlcle_green)
  (`ActorComponent.Activate` _ns_partlcle_green false))

(fn `UserConstructionScript`)