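; BP_ChangeLevel is an actor that switches between three streamed sublevels (Stage01, NewWorld, NewWorld1) using number keys 1 to 3.
; BeginPlay streams in Stage01 and enables input for the first player controller.
; Each key press shifts the target level into the current-level variable and sets the new target.
; The key release then unloads the current level and loads the target, both without blocking.
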(event `Key|One`
  (params (Key :type "Key Structure"))
  (:`Pressed`
    (set `self.CurLevel` (`self.MoveLevel`))
    (set `self.MoveLevel` "Stage01"))
  (:`Released`
    (`GameplayStatics.UnloadStreamLevel` (`KismetStringLibrary.Conv_StringToName` (`self.CurLevel`)) :!label _label)
    (`GameplayStatics.LoadStreamLevel` (`KismetStringLibrary.Conv_StringToName` (`self.MoveLevel`)) true)))

(event `Key|Two`
  (params (Key :type "Key Structure"))
  (:`Pressed`
    (set `self.CurLevel` (`self.MoveLevel`))
    (set `self.MoveLevel` "NewWorld"))
  (:`Released`
    (goto _label)))

(event `Key|Three`
  (params (Key :type "Key Structure"))
  (:`Pressed`
    (set `self.CurLevel` (`self.MoveLevel`))
    (set `self.MoveLevel` "NewWorld1"))
  (:`Released`
    (goto _label)))

(event `self.ReceiveBeginPlay`
  (`GameplayStatics.LoadStreamLevel` "Stage01" true)
  (set `self.CurLevel` "Stage01")
  (set `self.MoveLevel` "Stage01")
  (`self.EnableInput` (`GameplayStatics.GetPlayerController` 0)))

(fn `UserConstructionScript`)